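; Player character Blueprint for CrappyFlap that manages the player's HUD and input lock at game start.
; On BeginPlay it caches the CrappyFlapController, creates and displays the player widget, disables input and prints a debug string.
; Each Tick it polls the game mode's TimeUntilStart countdown and re-enables input while that value is zero.
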(event Custom|DisablePlayerInput
  (Input|DisableInput (Game|GetPlayerController 0)))

(event Custom|EnablePlayerInput
  (Input|EnableInput (Game|GetPlayerController 0)))

(event EventBeginPlay
  (bind _ascrappy_flap_controller (Utilities|Casting|CastToCrappyFlapController (Game|GetPlayerController 0)))
  (Variables|Default|SetPlayerController _ascrappy_flap_controller)
  (bind _returnvalue (UserInterface|CreateWidget "/Game/CrappyFlap/UI/PlayerWidget.PlayerWidget_C" (Variables|Default|GetPlayerController)))
  (bind _output_get (Variables|Default|SetPlayerWidget _returnvalue))
  (UserInterface|Viewport|AddtoViewport _output_get 0)
  (CallFunction|DisablePlayerInput)
  (Development|PrintString "Hello"))

(event Collision|EventActorBeginOverlap
  (params (OtherActor :type Actor%20Object%20Reference)))

(event EventTick
  (params (DeltaSeconds :type Float%20%28single-precision%29))
  (bind _ascrappy_flap_game_mode (Utilities|Casting|CastToCrappyFlapGameMode (Game|GetGameMode)))
  (if (== (Variables|/Script/Parteh.CrappyFlapGameMode|GetTimeUntilStart _ascrappy_flap_game_mode) 0)
    (CallFunction|EnablePlayerInput)))

(fn ConstructionScript)